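; CollectGuy is a collectible pickup for the Aria player character.
; On overlap with AriaCharacterBP it increments that character's NumCollect counter.
; It then deactivates one particle system, hides a second and disables the sphere's collision to prevent repeat pickups.
; A three-second timer then calls DIE to destroy the actor.
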(event `self.ReceiveActorBeginOverlap`
  (params (OtherActor :type "Actor Object Reference"))
  (bind _asaria_character_bp (cast `/Game/Blueprints/Player/AriaCharacterBP` OtherActor))
  (set `/Game/Blueprints/Player/AriaCharacterBP.NumCollect` (+ (`/Game/Blueprints/Player/AriaCharacterBP.NumCollect` _asaria_character_bp) 1) _asaria_character_bp)
  (`ActorComponent.Deactivate` (`self.ParticleSystem`))
  (`PrimitiveComponent.SetCollisionEnabled` (`self.Sphere`) "NoCollision")
  (`SceneComponent.SetVisibility` (`self.ParticleSystem1`) false false)
  (`KismetSystemLibrary.K2_SetTimerDelegate` (delegate `DIE`) 3.0))

(event `DIE`
  (`self.K2_DestroyActor`))

(fn `UserConstructionScript`)