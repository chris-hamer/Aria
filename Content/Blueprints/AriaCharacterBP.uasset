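; Aria player character with custom force-based movement and an auto-following camera, updated each Tick.
; Ground checks choose between trace and sweep hits by slope and step height, setting on-ground state for acceleration, curve-scaled deceleration and gravity.
; The spring arm yaws with sideways velocity and eases to default pitch, with manual look bypassed.
; The model faces camera-relative input when grounded and inherits yaw spin from rotating static mesh floors.
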(event `self.ReceiveTick`
  (params (DeltaSeconds :type "Float (single-precision)"))
  (`self.UpdateOTG`)
  (`self.MovementPhysics`)
  (`SceneComponent.K2_SetWorldTransform` (`self.ActualCamera`) (`SceneComponent.K2_GetComponentToWorld` (`self.FollowCamera`)) false false)
  (`self.CameraMovement`)
  (`self.DetermineNewFacingDirection`)
  (`self.TurnToFaceTargetDirection`))

(event `InputAxis|LookUpRate`
  (params (AxisValue :type "Float (single-precision)"))
  (bind (_controllercamerainput_x _controllercamerainput_y _controllercamerainput_z) (`KismetMathLibrary.BreakVector` (`self.ControllerCameraInput`)))
  (set `self.ControllerCameraInput` (`KismetMathLibrary.MakeVector` _controllercamerainput_x (* AxisValue 100.0 (`GameplayStatics.GetWorldDeltaSeconds`)) _controllercamerainput_z)))

(event `InputAxis|MoveRight`
  (params (AxisValue :type "Float (single-precision)"))
  (bind (_movementinput_x _movementinput_y _movementinput_z) (`KismetMathLibrary.BreakVector` (`self.MovementInput`)))
  (set `self.MovementInput` (`KismetMathLibrary.MakeVector` AxisValue _movementinput_y _movementinput_z)))

(event `InputAxis|LookUp`
  (params (AxisValue :type "Float (single-precision)"))
  (bind (_camerainput_x _camerainput_y _camerainput_z) (`KismetMathLibrary.BreakVector` (`self.CameraInput`)))
  (set `self.CameraInput` (`KismetMathLibrary.MakeVector` _camerainput_x AxisValue _camerainput_z)))

(event `InputAxis|MoveForward`
  (params (AxisValue :type "Float (single-precision)"))
  (bind (_movementinput_x _movementinput_y _movementinput_z) (`KismetMathLibrary.BreakVector` (`self.MovementInput`)))
  (set `self.MovementInput` (`KismetMathLibrary.MakeVector` _movementinput_x AxisValue _movementinput_z)))

(event `InputAxis|Turn`
  (params (AxisValue :type "Float (single-precision)"))
  (bind (_camerainput_x _camerainput_y _camerainput_z) (`KismetMathLibrary.BreakVector` (`self.CameraInput`)))
  (set `self.CameraInput` (`KismetMathLibrary.MakeVector` AxisValue _camerainput_y _camerainput_z)))

(event `InputAxis|TurnRate`
  (params (AxisValue :type "Float (single-precision)"))
  (bind (_controllercamerainput_x _controllercamerainput_y _controllercamerainput_z) (`KismetMathLibrary.BreakVector` (`self.ControllerCameraInput`)))
  (set `self.ControllerCameraInput` (`KismetMathLibrary.MakeVector` (* AxisValue 100.0 (`GameplayStatics.GetWorldDeltaSeconds`)) _controllercamerainput_y _controllercamerainput_z)))

(fn `AddMovementForce`
  (params (Force :type "Vector Structure"))
  (`self.AddMovementInput` (`KismetMathLibrary.Normal` Force) (`KismetMathLibrary.VSize` Force)))

(fn `CameraMovement`
  (bind (_camerainput_x _camerainput_y) (`KismetMathLibrary.BreakVector` (`self.CameraInput`)))
  (bind _actualcamera (`self.ActualCamera`))
  (bind (_camerainput_x_2 _camerainput_y_2) (`KismetMathLibrary.BreakVector` (`self.CameraInput`)))
  (bind (_relativerotation_roll _relativerotation_pitch) (`KismetMathLibrary.BreakRotator` (`SceneComponent.RelativeRotation` (`self.SpringArm`))))
  (bind (_relativerotation_roll_2 _relativerotation_pitch_2 _relativerotation_yaw) (`KismetMathLibrary.BreakRotator` (`SceneComponent.RelativeRotation` _actualcamera)))
  (`|ExecutionSequence`
    (:`then_0`
      (if true
        (`|ExecutionSequence`
          (:`then_0`
            (`SceneComponent.K2_AddRelativeRotation` (`self.SpringArm`) (`KismetMathLibrary.MakeRotator` 0.0 0.0 (* (/ (`KismetMathLibrary.Dot_VectorVector` (`self.GetVelocity2D`) (`self.GetCameraRight`)) (`self.MaxSpeed`)) (`GameplayStatics.GetWorldDeltaSeconds`) (`KismetMathLibrary.Abs` (.x (`self.MovementInput`))) 60.0)) false false))
          (:`then_2`
            (`SceneComponent.K2_SetRelativeRotation` (`self.SpringArm`) (`KismetMathLibrary.MakeRotator` (.roll (`SceneComponent.RelativeRotation` (`self.SpringArm`))) (`KismetMathLibrary.Lerp` (.pitch (`SceneComponent.RelativeRotation` (`self.SpringArm`))) (`self.DefaultPitch`) (* (`GameplayStatics.GetWorldDeltaSeconds`) 2.0)) (.yaw (`SceneComponent.RelativeRotation` (`self.SpringArm`)))) false false)))
        (elif (< (`KismetMathLibrary.Abs` (+ _relativerotation_pitch _camerainput_y)) 85.0)
          (`SceneComponent.K2_AddRelativeRotation` (`self.SpringArm`) (`KismetMathLibrary.MakeRotator` 0.0 _camerainput_y_2) false false)
          (`SceneComponent.K2_AddRelativeRotation` (`self.SpringArm`) (`KismetMathLibrary.MakeRotator` 0.0 0.0 _camerainput_x_2) false false))))
    (:`then_1`
      (`SceneComponent.K2_SetWorldTransform` (`self.ActualCamera`) (`KismetMathLibrary.TInterpTo` (`SceneComponent.K2_GetComponentToWorld` (`self.ActualCamera`)) (`SceneComponent.K2_GetComponentToWorld` (`self.FollowCamera`)) (`GameplayStatics.GetWorldDeltaSeconds`) 7.0) false false)
      (`SceneComponent.K2_SetRelativeRotation` _actualcamera (`KismetMathLibrary.MakeRotator` 0.0 _relativerotation_pitch_2 _relativerotation_yaw) false false))))

(fn `DECIDE`
  (params (NewParam :type "HitResult Structure") (NewParam1 :type "HitResult Structure"))
  (returns (NewParam2 :type "HitResult Structure"))
  (bind (_bblockinghit _binitialoverlap _time _distance _location _impactpoint _normal _impactnormal) (`GameplayStatics.BreakHitResult` NewParam))
  (bind (_bblockinghit_2 _binitialoverlap_2 _time_2 _distance_2 _location_2 _impactpoint_2 _normal_2 _impactnormal_2) (`GameplayStatics.BreakHitResult` NewParam1))
  (bind _returnvalue (<= (`KismetMathLibrary.DegCos` (`self.MaxSlopeAngle`)) (.z _impactnormal)))
  (return (select `bool` (and _returnvalue (<= (`KismetMathLibrary.DegCos` (`self.MaxSlopeAngle`)) (.z _impactnormal_2))) :`false` (select `bool` _returnvalue :`false` NewParam1 :`true` NewParam) :`true` (select `bool` (or (not (> (.z _impactpoint) (.z _impactpoint_2))) (> (`KismetMathLibrary.Abs` (`KismetMathLibrary.Dot_VectorVector` (- _impactpoint (`self.GetCapsuleBottom`)) (`self.GetUpDirection`))) (`AriaMovementComponent.MaxStepHeight` (`self.MovementComponent`)))) :`false` NewParam :`true` NewParam1))))

(fn `DetermineNewFacingDirection`
  (bind _movement_input (`self.GetAdjustedMovementInput`))
  (bind (_returnvalue_roll _returnvalue_pitch _returnvalue_yaw) (`KismetMathLibrary.BreakRotator` (`KismetMathLibrary.MakeRotFromX` (`KismetMathLibrary.Normal` _movement_input))))
  (if (and (> (`KismetMathLibrary.VSize` _movement_input) 0.001) (`AriaMovementComponent.OnTheGround` (`self.MovementComponent`)))
    (set `self.TargetDirection` (`KismetMathLibrary.MakeRotator` _returnvalue_roll _returnvalue_pitch (+ _returnvalue_yaw -90.0)))))

(fn `FlattenVelocity`
  (set `MovementComponent.Velocity` (`KismetMathLibrary.ProjectVectorOnToPlane` (`MovementComponent.Velocity` (`self.MovementComponent`)) (`self.GetUpDirection`)) (`self.MovementComponent`)))

(fn `GetAccelForce`
  (returns (Force :type "Vector Structure"))
  (return (* (`self.GetAdjustedMovementInput`) (`self.GetCurrentAccelRate`))))

(fn `GetAdjustedMovementInput`
  (returns (`Movement Input` :type "Vector Structure"))
  (return (+ (* (`self.GetCameraRight`) (.x (`KismetMathLibrary.ClampVectorSize` (`self.MovementInput`) 0.0 1.0))) (* (`self.GetCameraForward`) (.y (`KismetMathLibrary.ClampVectorSize` (`self.MovementInput`) 0.0 1.0))))))

(fn `GetCameraForward`
  (returns (Forward :type "Vector Structure"))
  (return (`KismetMathLibrary.Normal` (`KismetMathLibrary.ProjectVectorOnToPlane` (`SceneComponent.GetForwardVector` (`self.ActualCamera`)) (`self.GetUpDirection`)))))

(fn `GetCameraRight`
  (returns (Right :type "Vector Structure"))
  (return (`KismetMathLibrary.Normal` (`KismetMathLibrary.ProjectVectorOnToPlane` (`SceneComponent.GetRightVector` (`self.ActualCamera`)) (`self.GetUpDirection`)))))

(fn `GetCapsuleBottom`
  (returns (Bottom :type "Vector Structure"))
  (return (+ (`self.K2_GetActorLocation`) (* (* (`self.GetUpDirection`) -1.0) (`CapsuleComponent.CapsuleHalfHeight` (`self.CapsuleComponent`))))))

(fn `GetCurrentAccelRate`
  (returns (`Accel Rate` :type "Float (double-precision)"))
  (return (select `bool` (`AriaMovementComponent.OnTheGround` (`self.MovementComponent`)) :`false` (`self.AirAccelRate`) :`true` (`self.GroundAccelRate`))))

(fn `GetDecelForce`
  (returns (Force :type "Vector Structure"))
  (locals (DecelerationCurve :type "CurveFloat Object Reference" :default "CurveFloat'/Game/Blueprints/DecelCurve.DecelCurve'"))
  (bind _returnvalue (`KismetMathLibrary.ProjectVectorOnToPlane` (`MovementComponent.Velocity` (`self.MovementComponent`)) (`self.GetUpDirection`)))
  (bind _returnvalue_2 (/ (`KismetMathLibrary.VSize` _returnvalue) (`self.MaxSpeed`)))
  (return (* (* (`KismetMathLibrary.Normal` (* _returnvalue -1.0)) (select `bool` (`AriaMovementComponent.OnTheGround` (`self.MovementComponent`)) :`false` (/ (`self.AirAccelRate`) (`KismetMathLibrary.Lerp` 1.0 1.9 (`KismetMathLibrary.FClamp` (- _returnvalue_2 1.0)))) :`true` (`self.GroundAccelRate`))) (`CurveFloat.GetFloatValue` (`local.DecelerationCurve`) _returnvalue_2))))

(fn `GetEffectiveGravity`
  (returns (Gravity :type "Vector Structure"))
  (return (* (`self.Gravity`) (`self.CurrentGravityMultiplier`))))

(fn `GetUpDirection`
  (returns (Up :type "Vector Structure"))
  (return (0.0 0.0 1.0)))

(fn `GetVelocity2D`
  (returns (Velocity :type "Vector Structure"))
  (return (`KismetMathLibrary.ProjectVectorOnToPlane` (`MovementComponent.Velocity` (`self.MovementComponent`)) (`self.GetUpDirection`))))

(fn `MovementPhysics`
  (`|ExecutionSequence`
    (:`then_0`
      (`self.AddMovementForce` (`self.GetAccelForce`))
      (`self.AddMovementForce` (`KismetMathLibrary.ClampVectorSize` (`self.GetDecelForce`) 0.0 (/ (`KismetMathLibrary.VSize` (`MovementComponent.Velocity` (`self.MovementComponent`))) (`GameplayStatics.GetWorldDeltaSeconds`)))))
    (:`then_1`
      (if (`AriaMovementComponent.OnTheGround` (`self.MovementComponent`))
        (`self.FlattenVelocity`)
        (else
          (`self.AddMovementForce` (`self.GetEffectiveGravity`)))))))

(fn `TurnToFaceTargetDirection`
  (bind (_groundhitresult_bblockinghit _groundhitresult_binitialoverlap _groundhitresult_time _groundhitresult_distance _groundhitresult_location _groundhitresult_impactpoint _groundhitresult_normal _groundhitresult_impactnormal _groundhitresult_physmat _groundhitresult_hitactor _groundhitresult_hitcomponent) (`GameplayStatics.BreakHitResult` (`self.GroundHitResult`)))
  (`|ExecutionSequence`
    (:`then_0`
      (if (and (`KismetSystemLibrary.IsValid` _groundhitresult_hitactor) (`KismetSystemLibrary.IsValid` _groundhitresult_hitcomponent) (== (`GameplayStatics.GetObjectClass` _groundhitresult_hitcomponent) "/Script/Engine.StaticMesh"))
        (bind _returnvalue (`PrimitiveComponent.GetPhysicsAngularVelocityInDegrees` _groundhitresult_hitcomponent "None"))
        (`SceneComponent.K2_AddLocalRotation` (`self.Model`) (`KismetMathLibrary.MakeRotator` 0.0 0.0 (* (`KismetMathLibrary.Dot_VectorVector` _returnvalue (`self.GetUpDirection`)) (`GameplayStatics.GetWorldDeltaSeconds`))) false false)))
    (:`then_1`
      (`self.TurnModel`))))

(fn `UpdateOTG`
  (locals (TraceLength :type "Float (double-precision)") (PlayerBottom :type "Vector Structure") (GroundTraceHit :type "HitResult Structure") (CanStand :type Boolean) (AirTraceLength :type "Float (double-precision)") (GroundTraceLength :type "Float (double-precision)") (GroundSweepHit :type "HitResult Structure"))
  (set `self.WasOnTheGround` (`AriaMovementComponent.OnTheGround` (`self.MovementComponent`)))
  (bind _returnvalue (`AriaMovementComponent.DoGroundSweep` (`self.MovementComponent`)))
  (bind _output_get (set `local.GroundSweepHit` _returnvalue))
  (bind _returnvalue_2 (`AriaMovementComponent.DoGroundTrace` (`self.MovementComponent`)))
  (bind _output_get_2 (set `local.GroundTraceHit` _returnvalue_2))
  (set `self.PrevGroundHitResult` (`self.GroundHitResult`))
  (bind _returnvalue_3 (`AriaMovementComponent.DoGroundTraceSweep` (`self.MovementComponent`)))
  (bind _output_get_3 (set `local.GroundTraceHit` (`self.DECIDE` (`local.GroundTraceHit`) _returnvalue_3)))
  (`|ExecutionSequence`
    (:`then_0`
      (bind (_bblockinghit _binitialoverlap _time _distance _location _impactpoint) (`GameplayStatics.BreakHitResult` _output_get))
      (bind _output_get_4 (set `AriaMovementComponent.OnTheGround` (and (or (`GameplayStatics.BreakHitResult` _output_get_3) (`.bInitialOverlap` (`GameplayStatics.BreakHitResult` _output_get_3))) (<= (`KismetMathLibrary.DegCos` (`self.MaxSlopeAngle`)) (.z (`.ImpactNormal` (`GameplayStatics.BreakHitResult` _output_get_3)))) (and _bblockinghit (<= (`KismetMathLibrary.Abs` (`KismetMathLibrary.Dot_VectorVector` (- _impactpoint (`self.GetCapsuleBottom`)) (`self.GetUpDirection`))) (`AriaMovementComponent.MaxStepHeight` (`self.MovementComponent`)))) true) (`self.MovementComponent`)))
      (if _output_get_4
        (set `self.CurrentFloorActor` (`.HitActor` (`GameplayStatics.BreakHitResult` _output_get_3)))
        (bind _returnvalue_4 (`AriaMovementComponent.DoGroundTraceSweep` (`self.MovementComponent`)))
        (set `AriaMovementComponent.GroundSweep` (`self.DECIDE` (`local.GroundTraceHit`) _returnvalue_4) (`self.MovementComponent`))
        (`AriaMovementComponent.AdjustFloor` (`self.MovementComponent`))))
    (:`then_1`
      (set `self.GroundHitResult` (`AriaMovementComponent.GroundSweep` (`self.MovementComponent`))))))

(fn `UserConstructionScript`)