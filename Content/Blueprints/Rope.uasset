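; Climbable-style rope actor that switches AriaCharacterBP into a dedicated player state while the character overlaps it.
; On overlap begin it sets that state, rotates the model to the target direction, and teleports the character slightly behind the rope along the model's forward vector, keeping its height.
; On overlap end it restores another state, only if the character is still in the rope state.
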(event `self.ReceiveActorBeginOverlap`
  (params (OtherActor :type "Actor Object Reference"))
  (bind _asaria_character_bp (cast `/Game/Blueprints/Player/AriaCharacterBP` OtherActor))
  (`/Game/Blueprints/Player/AriaCharacterBP.SetPlayerState` _asaria_character_bp "NewEnumerator15")
  (bind _model (`AriaCharacter.Model` _asaria_character_bp))
  (`SceneComponent.K2_SetWorldRotation` _model (`AriaCharacter.TargetDirection` _asaria_character_bp) false false)
  (bind (_returnvalue_x _returnvalue_y) (`KismetMathLibrary.BreakVector` (- (`self.K2_GetActorLocation`) (* (`SceneComponent.GetForwardVector` _model) 15.0))))
  (bind (_returnvalue_x_2 _returnvalue_y_2 _returnvalue_z) (`KismetMathLibrary.BreakVector` (`self.K2_GetActorLocation` _asaria_character_bp)))
  (`self.K2_SetActorLocation` _asaria_character_bp (`KismetMathLibrary.MakeVector` _returnvalue_x _returnvalue_y _returnvalue_z) false true))

(event `self.ReceiveActorEndOverlap`
  (params (OtherActor :type "Actor Object Reference"))
  (bind _asaria_character_bp (cast `/Game/Blueprints/Player/AriaCharacterBP` OtherActor))
  (if (== (`/Game/Blueprints/Player/AriaCharacterBP.CurrentPlayerState` _asaria_character_bp) (`BlueprintMapLibrary.Map_Find` (`/Game/Blueprints/Player/AriaCharacterBP.PlayerStates` _asaria_character_bp) "NewEnumerator15"))
    (`/Game/Blueprints/Player/AriaCharacterBP.SetPlayerState` _asaria_character_bp "NewEnumerator0")))

(fn `UserConstructionScript`)